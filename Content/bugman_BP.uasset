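; Bugman is a 2D-sprite enemy pawn that wanders at random and can be killed by sword hits.
; Tick drives everything: it destroys the actor at zero HP and, after random delays, sends AI moves to reachable points nearby.
; While moving, a resettable DoOnce with delays bobs the paper sprite up and down.
; Sword overlaps on the hit box subtract the weapon's damage and trigger blood.
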(event `self.ReceiveTick`
  (params (DeltaSeconds :type "Float (single-precision)"))
  (bind _papersprite (`self.PaperSprite`))
  (`|ExecutionSequence`
    (:`then_0`
      ;[1 1 1] Death
      (if (<= (`self.HP`) 0)
        (`self.K2_DestroyActor`)))
    (:`then_1`
      ;[1 1 1] Roam AI
      (`KismetSystemLibrary.Delay` (`KismetMathLibrary.RandomFloatInRange` 1.0 5.0))
      (set `self.IsMoving?` true)
      (`|AIMoveTo` self (`NavigationSystemV1.K2_GetRandomReachablePointInRadius` (`self.K2_GetActorLocation`) 1500.0 null null) null
        (:`OnSuccess`
          _)
        (:`OnFail`
          _))
      (set `self.IsMoving?` false))
    (:`then_2`
      (if (`self.IsMoving?`)
        (`/Engine/EditorBlueprintResources/StandardMacros.DoOnce` false :!label _label
          (:`Completed`
            (`SceneComponent.K2_SetRelativeLocation` _papersprite (0.0 0.0 10.0) false false)
            (`KismetSystemLibrary.Delay` 0.2)
            (`SceneComponent.K2_SetRelativeLocation` _papersprite (0.0 0.0 0.0) false false)
            (`KismetSystemLibrary.Delay` 0.2)
            (goto _label :!via `Reset`)))
        (else
          (`SceneComponent.K2_SetRelativeLocation` (`self.PaperSprite`) (0.0 0.0 0.0) false false))))))

(event `self.HitBox.OnComponentBeginOverlap`
  (params (OverlappedComponent :type "PrimitiveComponent Object Reference") (OtherActor :type "Actor Object Reference") (OtherComp :type "PrimitiveComponent Object Reference") (OtherBodyIndex :type Integer) (bFromSweep :type Boolean) (SweepResult :type "HitResult Structure (by ref)"))
  (bind _assword (cast `/Game/Sword` OtherActor))
  (set `self.HP` (- (`self.HP`) (`/Game/Sword.Damage` _assword)))
  (`ActorComponent.Activate` (`self.blood`) true)
  (`KismetSystemLibrary.PrintString` "BugMan Hurt"))

(fn `UserConstructionScript`)